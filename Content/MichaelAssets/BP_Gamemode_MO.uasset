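; BP_Gamemode_MO is the game mode for a ship game, enforcing a circular play-area boundary formed by a nebula.
; BeginPlay caches the player ship, its spawn point and the game state, then starts the game state and refreshes the shield HUD.
; Each Tick measures the ship's 2D distance from world origin to toggle the nebula warning, drain shields inside the nebula, or return it to spawn beyond the maximum distance.
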(event EventBeginPlay
  (bind _asbp_player_mo (Utilities|Casting|CastToBP_Player_MO (Game|Player|GetPlayerPawn 0)))
  (bind _output_get (Variables|Default|SetPlayerShip _asbp_player_mo))
  (Variables|Default|SetSpawnPoint (Transformation|GetActorLocation _output_get))
  (bind _asgs_game_state_mo (Utilities|Casting|CastToGS_GameState_MO (Game|GetGameState)))
  (bind _output_get_2 (Variables|Default|SetCurrentGameState _asgs_game_state_mo))
  (Default|Start _output_get_2)
  (Default|UpdateShields (Variables|/Game/MichaelAssets/BP_HUD_MO.BP_HUD_MO_C|GetMainHUD_MO (Variables|Default|GetHUD))))

(event EventTick
  (params (DeltaSeconds :type Float%20%28single-precision%29))
  (bind _playership (Variables|Default|GetPlayerShip))
  (bind _hud (Variables|Default|GetHUD))
  (bind _returnvalue (Transformation|GetActorLocation _playership))
  (bind _mainhud_mo (Variables|/Game/MichaelAssets/BP_HUD_MO.BP_HUD_MO_C|GetMainHUD_MO _hud))
  (bind (_x _y) (Math|Vector|BreakVector _returnvalue))
  (bind _returnvalue_2 (Math|Vector2D|MakeVector2D _x _y))
  (bind _returnvalue_3 (Math|Vector|Distance2D(Vector) :V2 _returnvalue_2))
  (if (> _returnvalue_3 (Variables|Default|GetNebulaWarningDistance))
    (Default|UpdateInsideNebula _mainhud_mo true)
    (else
      (Default|UpdateInsideNebula _mainhud_mo false)))
  (if (> _returnvalue_3 (Variables|Default|GetNebulaDistance))
    (if (> _returnvalue_3 (Variables|Default|GetMaxDistance))
      (Transformation|SetActorLocation (Variables|Default|GetPlayerShip) (Variables|Default|GetSpawnPoint) false false)
      (else
        (Class|ReturntoAlderaanGameMode|ModifyShieldAmount -0.2)
        (Default|UpdateShields (Variables|/Game/MichaelAssets/BP_HUD_MO.BP_HUD_MO_C|GetMainHUD_MO (Variables|Default|GetHUD)))))))

(fn ConstructionScript)