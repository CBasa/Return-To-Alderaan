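; Player ship Blueprint that handles collision damage, look yaw and the game over screen.
; Capsule hits send the collision object's damage, or a default, to the game mode's shield, then a timed invincibility window blocks further hits.
; BeginPlay restores game-only input after a restart.
; The 0 key calls GameOver, which pauses the game and shows the game over widget with UI-only input.
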(event OnComponentHit(CapsuleComponent)
  (params (HitComponent :type Primitive%20Component%20Object%20Reference) (OtherActor :type Actor%20Object%20Reference) (OtherComp :type Primitive%20Component%20Object%20Reference) (NormalImpulse :type Vector :default "0, 0, 0") (Hit :type Hit%20Result%20Structure%20%28by%20ref%29))
  ;[1 1 1] Collision Function
  (if (not (Variables|Default|GetInvincible))
    (Variables|Default|SetInvincible true)
    (bind _asreturn_to_alderaan_game_mode_combined (Utilities|Casting|CastToReturnToAlderaanGameMode_Combined (Game|GetGameMode))
      (:then
        (bind _ascpp_collision_object_mo (Utilities|Casting|CastToCPP_CollisionObject_MO OtherActor)
          (:then
            (Class|ReturntoAlderaanGameMode|ModifyShieldAmount _asreturn_to_alderaan_game_mode_combined (Variables|/Script/ReturnToAlderaan.CPP_CollisionObject_MO|GetcollisionDamage _ascpp_collision_object_mo)))
          (:CastFailed
            (Class|ReturntoAlderaanGameMode|ModifyShieldAmount _asreturn_to_alderaan_game_mode_combined (Variables|Default|GetCollision%20Damage))))
        ;[1 1 1] Resets Player Invincibility
        (Utilities|FlowControl|Delay (Variables|Default|GetInvincibilityTime))
        (Variables|Default|SetInvincible false))
      (:CastFailed
        (Development|PrintString "Colision cast fail on player ship.")))))

(event Input|EnhancedActionEvents|EnhancedInputActionIA_Look
  (params (ActionValue :type Vector%202D%20Structure) (ElapsedSeconds :type Float%20%28double-precision%29) (TriggeredSeconds :type Float%20%28double-precision%29) (InputAction :type Input%20Action%20Object%20Reference :default "/Game/ThirdPerson/Input/Actions/IA_Look.IA_Look"))
  ;[1 1 1] Overrides Ship rotation
  (Pawn|Input|AddControllerYawInput (* (.x ActionValue) 0.5)))

(event EventBeginPlay
  (bind _returnvalue (Game|GetPlayerController 0))
  ;[1 1 1] Reset Input Mode After Restart
  (Variables|/Script/Engine.PlayerController|SetbShowMouseCursor _returnvalue false)
  (Input|SetInputModeGameOnly _returnvalue false)
  ;[1 1 1] Resets Player Invincibility
  (Utilities|FlowControl|Delay (Variables|Default|GetInvincibilityTime))
  (Variables|Default|SetInvincible false))

(event Input|KeyboardEvents|0
  (params (Key :type Key%20Structure :default "None"))
  ;[1 1 1] Trigger Game Over Screen
  (:Pressed
    (CallFunction|GameOver)))

(fn ConstructionScript)

(fn GameOver
  (bind _returnvalue (Game|GetPlayerController 0))
  (Game|SetGamePaused true)
  (bind _returnvalue_2 (UserInterface|CreateWidget "/Game/UI/GameOver/WBP_GameOverScreen_CB.WBP_GameOverScreen_CB_C"))
  (UserInterface|Viewport|AddtoViewport _returnvalue_2 0)
  (Variables|/Script/Engine.PlayerController|SetbShowMouseCursor _returnvalue true)
  (Input|SetInputModeUIOnly _returnvalue _returnvalue_2 "DoNotLock" false))