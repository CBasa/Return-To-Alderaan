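; BP_BlackHole_RJ is a black hole actor that shows a UI screen when the shuttle is destroyed by a black hole.
; BeginPlay creates the WBP_Blackhole_RJ widget and casts the game mode without using the result.
; Tick polls ShuttleDestroyedByBlackhole on GameStateBase_RJ and, every frame it is true, calls AddToViewport and shows the mouse cursor.
; The Blueprint only reads that flag and has no active overlap logic.
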(event EventBeginPlay
  (bind _returnvalue (UserInterface|CreateWidget "/Game/UI/GameOver/WBP_Blackhole_RJ.WBP_Blackhole_RJ_C"))
  (Variables|Default|SetBlackholeWidget _returnvalue)
  (Utilities|Casting|CastToReturnToAlderaanGameMode_RJ (Game|GetGameMode)))

(event Collision|EventActorBeginOverlap
  (params (OtherActor :type Actor%20Object%20Reference)))

(event EventTick
  (params (DeltaSeconds :type Float%20%28single-precision%29))
  (bind _asgame_state_base_rj (Utilities|Casting|CastToGameStateBase_RJ (Game|GetGameState)))
  (if (Variables|/Script/ReturnToAlderaan.GameStateBase_RJ|GetShuttleDestroyedByBlackhole _asgame_state_base_rj)
    (UserInterface|Viewport|AddtoViewport (Variables|Default|GetBlackholeWidget) 0)
    (Variables|/Script/Engine.PlayerController|SetbShowMouseCursor (Game|GetPlayerController 0) true)))

(fn ConstructionScript)