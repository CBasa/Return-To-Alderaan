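; BP_Player_MO_RJ is a player character Blueprint with a timed speed boost, horizontal-only look input and suppressed jumping.
; BeginPlay caches the regular max speed, and Tick polls SpeedBoostActive on MyGameStateBase_RJ to apply BoostedMaxSpeed.
; A Delay inside Tick restores the cached speed after SpeedBoostTimeToLive, without clearing the flag here.
; Jump input calls StopJumping and prints a notice, while look input adds scaled controller yaw.
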(event Input|EnhancedActionEvents|EnhancedInputActionIA_Jump
  (params (ActionValue :type Boolean) (ElapsedSeconds :type Float%20%28double-precision%29) (TriggeredSeconds :type Float%20%28double-precision%29) (InputAction :type Input%20Action%20Object%20Reference :default "/Game/ThirdPerson/Input/Actions/IA_Jump.IA_Jump"))
  (Character|StopJumping (Class|CharacterMovementComponent|GetCharacterOwner (Variables|Character|GetCharacterMovement)))
  (Development|PrintText "Jump Ignored"))

(event Input|EnhancedActionEvents|EnhancedInputActionIA_Look
  (params (ActionValue :type Vector%202D%20Structure) (ElapsedSeconds :type Float%20%28double-precision%29) (TriggeredSeconds :type Float%20%28double-precision%29) (InputAction :type Input%20Action%20Object%20Reference :default "/Game/ThirdPerson/Input/Actions/IA_Look.IA_Look"))
  (Pawn|Input|AddControllerYawInput (* (.x ActionValue) 0.5)))

(event EventBeginPlay
  (Variables|Default|SetRegularMaxSpeed (Class|MovementComponent|GetMaxSpeed (Variables|Character|GetCharacterMovement))))

(event Collision|EventActorBeginOverlap
  (params (OtherActor :type Actor%20Object%20Reference)))

(event EventTick
  (params (DeltaSeconds :type Float%20%28single-precision%29))
  (bind _asmy_game_state_base_rj (Utilities|Casting|CastToMyGameStateBase_RJ (Game|GetGameState)))
  (if (Variables|/Script/ReturnToAlderaan.GameStateBase_RJ|GetSpeedBoostActive _asmy_game_state_base_rj)
    (Variables|/Script/Engine.CharacterMovementComponent|SetMaxWalkSpeed (Variables|Character|GetCharacterMovement) (Variables|Default|GetBoostedMaxSpeed))
    (Utilities|FlowControl|Delay (Variables|Default|GetSpeedBoostTimeToLive))
    (Variables|/Script/Engine.CharacterMovementComponent|SetMaxWalkSpeed (Variables|Character|GetCharacterMovement) (Variables|Default|GetRegularMaxSpeed))))

(fn ConstructionScript)